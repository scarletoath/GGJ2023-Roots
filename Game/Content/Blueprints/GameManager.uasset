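; GameManager Blueprint that keeps a running score for each score type in a Scores array indexed by the enum value.
; An Init event sizes the array from the enum's entry count, using an array set with size-to-fit.
; ChangeScore adds a delta to the value from GetScore, writes it back and returns the new total.
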(event EventInit
  ;[1 1 1] Initialize Scores array to correct size
  (bind _result (Math|Integer|DecrementInt (|GetNumEnumEntries))
    (:%20%20
      (Utilities|Array|SetArrayElem (Variables|Default|GetScores) _result 0 true))))

(fn ChangeScore
  (params (ScoreType :type ScoreType%20Enum :default "NewEnumerator0") (DeltaScore :type Integer))
  (bind _score (CallFunction|GetScore ScoreType))
  (Utilities|Array|SetArrayElem (Variables|Default|GetScores) (Math|Conversions|ToInteger(Byte) ScoreType) (+ DeltaScore _score) true)
  (return (+ DeltaScore _score)))

(fn GetScore
  (params (ScoreType :type ScoreType%20Enum :default "NewEnumerator0"))
  (return (Utilities|Array|Get(acopy) (Variables|Default|GetScores) (Math|Conversions|ToInteger(Byte) ScoreType))))