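; BP_BGActor_Bunny is a background bunny for the DyeMaker minigame that squashes and stretches in time to a fixed tempo.
; BeginPlay derives a half-beat interval from 72 BPM.
; Tick linearly eases Z scale between two bounce values, swapping them after each interval to reverse direction.
; Random repositioning and position-list logic is left disconnected, so the actor never moves.
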(event EventBeginPlay
  (bind _returnvalue (Math|Random|RandomFloatinRange 1e+01 2e+01))
  (Variables|Default|SettimeTillBeat (Utilities|Operators|Divide 6e+01 72.0 2.0))
  (Variables|Default|SetcurrentPos (Transformation|GetActorLocation))
  (Variables|Default|SetnewPos (Math|Vector|MakeVector _returnvalue (.Y (Math|Vector|BreakVector (Variables|Default|GetcurrentPos))) _returnvalue)))

(event Collision|EventActorBeginOverlap
  (params (OtherActor :type Actor%20Object%20Reference)))

(event EventTick
  (params (DeltaSeconds :type Float%20%28single-precision%29))
  (Variables|Default|SetcurrentTime (+ DeltaSeconds (Variables|Default|GetcurrentTime)))
  (Utilities|FlowControl|Sequence
    (:then_0
      (if (<= (Variables|Default|GetcurrentTime) (Variables|Default|GettimeTillBeat))
        (Transformation|SetActorScale3D (Math|Vector|MakeVector 1.0 1.0 (Math|Interpolation|Ease "Linear" (/ (Variables|Default|GetcurrentTime) (Variables|Default|GettimeTillBeat)) (Variables|Default|GetstartBounce) (Variables|Default|GetendBounce))))
        (else
          (Variables|Default|SetcurrentTime 0.0)
          (Variables|Default|SetsaveValue (Variables|Default|GetstartBounce))
          (Variables|Default|SetstartBounce (Variables|Default|GetendBounce))
          (Variables|Default|SetendBounce (Variables|Default|GetsaveValue)))))))

(fn ConstructionScript)