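; Beat marker for the DyeMaker minigame that measures how far a press lands from its beat.
; When not OnMap it spawns an overlay at its location, and once EnableScoreOnDelay starts the countdown, Tick eases its scale toward 1 and accumulates lateness after zero.
; Kaboom spawns score and FX actors, reports the signed timing offset on success or the remaining countdown on failure, then destroys itself and the overlay.
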(event EventBeginPlay
  (if (not (Variables|Default|GetonMap))
    (bind _returnvalue (Game|SpawnActorfromClass "/Game/Blueprints/MiniGames/DyeMaker/BP_BeatIndicatorOverlay.BP_BeatIndicatorOverlay_C" (Transformation|GetActorTransform) "Undefined" 0 0))
    (Variables|Default|Setoverlay _returnvalue)))

(event Collision|EventActorBeginOverlap
  (params (OtherActor :type Actor%20Object%20Reference)))

(event EventTick
  (params (DeltaSeconds :type Float%20%28single-precision%29))
  (if (not (Variables|Default|GetonMap))
    (if (Variables|Default|GetcountdownToScore)
      (bind _output_get (Variables|Default|SetcountdownToScoreEnabled (- (Variables|Default|GetcountdownToScoreEnabled) DeltaSeconds)))
      (bind _output_get_2 (Variables|Default|SetstartScale (Math|Interpolation|FInterpTo (Variables|Default|GetstartScale) 1.0 DeltaSeconds 1.0)))
      (Transformation|SetActorScale3D (Math|Vector|MakeVector _output_get_2 _output_get_2 _output_get_2))
      (if (<= _output_get 0.0)
        (Variables|Default|SetscoreDelay (+ (Variables|Default|GetscoreDelay) DeltaSeconds))))))

(fn ConstructionScript)

(fn Kaboom
  (params (success :type Boolean))
  (bind _returnvalue (Game|SpawnActorfromClass "/Game/Blueprints/MiniGames/DyeMaker/BP_Score.BP_Score_C" (Transformation|GetActorTransform) "Undefined" 0 0))
  (Utilities|String|LogString "KABOOM!")
  (bind _returnvalue_2 (Game|SpawnActorfromClass "/Game/Blueprints/MiniGames/DyeMaker/BP_FX_Dyemaker.BP_FX_Dyemaker_C" (Transformation|GetActorTransform) "Undefined" 0 0))
  (Default|SetFX _returnvalue_2 success)
  (if success
    (bind _returnvalue_3 (CallFunction|Score))
    (LocalVariables|SetreturnScoreDelay _returnvalue_3)
    (else
      (LocalVariables|SetreturnScoreDelay (Variables|Default|GetcountdownToScoreEnabled))))
  (Default|UpdateScore _returnvalue (LocalVariables|GetreturnScoreDelay) success)
  (Actor|DestroyActor (Variables|Default|Getoverlay))
  (Actor|DestroyActor)
  (return (LocalVariables|GetreturnScoreDelay)))

(fn Score
  (if (> (Variables|Default|GetcountdownToScoreEnabled) 0.0)
    (bind _output_get (LocalVariables|SetfinalDelay (- (Variables|Default|GetscoreDelay) (Variables|Default|GetcountdownToScoreEnabled))))
    (Utilities|String|LogString (Utilities|String|Append "EARLY PRESS... by" (Utilities|String|ToString(Float) _output_get)))
    (else
      (bind _output_get_2 (LocalVariables|SetfinalDelay (Variables|Default|GetscoreDelay)))
      (Utilities|String|LogString (Utilities|String|Append "SCORE DELAY BY" (Utilities|String|ToString(Float) _output_get_2)))))
  (return (LocalVariables|GetfinalDelay)))

(fn EnableScoreonDelay
  (params (delay :type Float%20%28double-precision%29))
  (Variables|Default|SetcountdownToScore true)
  (Variables|Default|SetcountdownToScoreEnabled delay))