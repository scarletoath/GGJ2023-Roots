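; 2D beat indicator actor for the DyeMaker rhythm minigame, showing the key or key combo for one timed beat.
; EnableBeat sets the perfect and end timestamps, starts a gentle zoom on Tick, and shows keys as joined text or centered, scaled-down sprites created at runtime.
; Kaboom resolves the beat: it plays a splash, spawns FX and score actors, scores by offset from perfect time (full window on failure), then destroys itself.
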(event EventBeginPlay
  ;[1 1 1] Hide stuff until ready
  (CallFunction|EnableHighlight false)
  (Rendering|SetVisibility (Variables|Default|GetKEY%20TO%20PRESS_Text) false false))

(event Collision|EventActorBeginOverlap
  (params (OtherActor :type Actor%20Object%20Reference)))

(event EventTick
  (params (DeltaSeconds :type Float%20%28single-precision%29))
  ;[1 1 1] Zoom In Gently once Scoring Enabled
  (if (Variables|Default|GetscoreEnabled)
    (bind _output_get (Variables|Default|SetstartScale (Math|Interpolation|FInterpTo (Variables|Default|GetstartScale) 1.0 DeltaSeconds 1.0)))
    (Transformation|SetActorScale3D (Math|Conversions|ToVector(Float) _output_get))))

(fn ConstructionScript)

(fn Kaboom
  (params (success :type Boolean))
  (bind _returnvalue (Transformation|GetActorTransform))
  (Utilities|FlowControl|Sequence
    (:then_0
      (LocalVariables|SetisSuccess success)
      (Variables|Default|SetscoreEnabled false))
    (:then_1
      (Audio|PlaySound2D "/Game/Audio/DyeMaker/Splash_WaterEmerge04.Splash_WaterEmerge04" 0.2 1.0 0.6 0 0))
    (:then_2
      ;[1 1 1] Spawners
      (bind _returnvalue_2 (Game|SpawnActorfromClass "/Game/Blueprints/MiniGames/DyeMaker/BP_Score.BP_Score_C" _returnvalue "Undefined" 0 0))
      (LocalVariables|SetscoreActor _returnvalue_2)
      (Utilities|String|LogString "KABOOM!"))
    (:then_3
      (bind _returnvalue_3 (Game|SpawnActorfromClass "/Game/Blueprints/MiniGames/DyeMaker/BP_FX_Dyemaker.BP_FX_Dyemaker_C" _returnvalue "Undefined" 0 0))
      (Default|SetFX _returnvalue_3 (LocalVariables|GetisSuccess)))
    (:then_4
      ;[1 1 1] Calculate Score
      (LocalVariables|Setdelay (Math|Float|SelectFloat (CallFunction|GetDelay) (- (Variables|Default|GettimeBeatOver) (Variables|Default|GettimePerfectBeat)) (LocalVariables|GetisSuccess))))
    (:then_5
      (Default|UpdateScore (LocalVariables|GetscoreActor) (LocalVariables|Getdelay) (LocalVariables|GetisSuccess)))
    (:then_6
      (Actor|DestroyActor)
      (return (LocalVariables|Getdelay)))))

(fn GetDelay
  (bind _returnvalue (Utilities|Time|GetGameTimeinSeconds))
  (bind _timeperfectbeat (Variables|Default|GettimePerfectBeat))
  (bind _returnvalue_2 (- _returnvalue _timeperfectbeat))
  ;[1 1 1] Debug log
  (Development|PrintString (Utilities|String|Append (Utilities|String|SelectString "EARLY PRESS... by" "SCORE DELAY BY" (<= _returnvalue_2 0.0)) (Utilities|String|ToString(Float) _returnvalue_2)) true true "(R=0.000000,G=0.660000,B=1.000000,A=1.000000)" 1e+01)
  (return _returnvalue_2))

(fn EnableBeat
  (params (delay :type Float%20%28double-precision%29) (beatDuration :type Float%20%28double-precision%29) (activationKeys :type Array%20of%20Key%20Structures :default "None") (showText :type Boolean))
  (bind _returnvalue (Utilities|Time|GetGameTimeinSeconds))
  (bind _returnvalue_2 (+ delay _returnvalue))
  (Utilities|FlowControl|Sequence
    (:then_0
      ;[1 1 1] Configure Scoring Parameters
      (Variables|Default|SetscoreEnabled true)
      (Variables|Default|SettimePerfectBeat _returnvalue_2)
      (Variables|Default|SettimeBeatOver (+ _returnvalue_2 beatDuration)))
    (:then_1
      ;[1 1 1] Update Key(s) Display
      (Variables|Default|SetactivationKeys activationKeys)
      (CallFunction|UpdateDisplayedKeys showText))))

(fn GetActivationKeys
  (return (Variables|Default|GetactivationKeys)))

(fn EnableHighlight
  (params (IsHighlighted :type Boolean))
  (Rendering|SetVisibility (Variables|Default|GetHighlight) IsHighlighted true))

(fn UpdateDisplayedKeys
  (params (useText :type Boolean))
  (bind _spriteroot (Variables|Default|GetSpriteRoot))
  (bind _activationkeys (Variables|Default|GetactivationKeys))
  (bind _returnvalue (Utilities|Array|Length _activationkeys))
  (if useText
    ;[1 1 1] Text
    (for _array_element (Variables|Default|GetactivationKeys)
      (Utilities|Array|Add (LocalVariables|GetkeyLabels) (.Label (CallFunction|GetKeyDisplayInfo _array_element))))
    (Rendering|Components|TextRender|SetText (Variables|Default|GetKEY%20TO%20PRESS_Text) (Utilities|Text|ToText(String) (Utilities|String|JoinStringArray (LocalVariables|GetkeyLabels) "+")))
    (else
      ;[1 1 1] Sprite
      (for (_array_element_2 _array_index) _activationkeys
        (bind _new_sprite (Utilities|CreateSpriteforIndex _array_index _returnvalue 7e+01)
          (:execOut
            (Rendering|Components|Sprite|SetSprite _new_sprite (.Sprite (CallFunction|GetKeyDisplayInfo _array_element_2))))))
      ;;[1 1 1] Scale down to fit
      (Transformation|SetRelativeScale3D _spriteroot (Math|Conversions|ToVector(Float) (/ 1.0 (Math|Conversions|ToFloat(Integer) _returnvalue))))
      (Rendering|SetVisibility _spriteroot true true))))

(fn IsBeatOver
  (return (>= (Utilities|Time|GetGameTimeinSeconds) (Variables|Default|GettimeBeatOver))))