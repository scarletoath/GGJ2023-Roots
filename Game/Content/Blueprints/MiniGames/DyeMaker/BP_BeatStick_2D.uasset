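; BP_BeatStick_2D is the moving beat marker for the 2D DyeMaker minigame.
; It reads its waypoint actors from GM_Dyemaker_2D, retrying on Tick while none are available.
; Tick linearly interpolates its location from one waypoint to the next over a hardcoded 72 BPM beat, looping through the list.
; On each beat it advances the waypoint index and restarts the NGSplash effect.
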(event EventBeginPlay
  (bind _asgm_dyemaker_2d (Utilities|Casting|CastToGM_Dyemaker_2D (Game|GetGameMode)))
  (Variables|Default|SetGameMode _asgm_dyemaker_2d)
  (CallFunction|Initialize))

(event Collision|EventActorBeginOverlap
  (params (OtherActor :type Actor%20Object%20Reference)))

(event EventTick
  (params (DeltaSeconds :type Float%20%28single-precision%29))
  (bind _gamemode (Variables|Default|GetGameMode))
  (bind _positions (Variables|/Game/Blueprints/MiniGames/DyeMaker/GM_Dyemaker_2D.GM_Dyemaker_2D_C|GetPositions _gamemode))
  (if (Variables|Default|GethasPositions) :!label _label
    (Variables|Default|SetcurrentTime (+ DeltaSeconds (Variables|Default|GetcurrentTime)))
    (if (<= (Variables|Default|GetcurrentTime) (Variables|Default|GettimeTillBeat))
      (Transformation|SetActorLocation (.Location (Math|Transform|BreakTransform (Math|Interpolation|Ease "Linear" (/ (Variables|Default|GetcurrentTime) (Variables|Default|GettimeTillBeat)) (Transformation|GetActorTransform (Utilities|Array|Get(acopy) _positions (Variables|Default|GetcurrentPos))) (Transformation|GetActorTransform (Utilities|Array|Get(acopy) _positions (Math|Integer|SelectInt (+ (Variables|Default|GetcurrentPos) 1) 0 (< (+ (Variables|Default|GetcurrentPos) 1) (Variables|Default|GetmaxPos)))))))) false false)
      (else
        (Variables|Default|SetcurrentTime 0.0)
        (bind _result (Math|Integer|IncrementInt (Variables|Default|GetcurrentPos))
          (:%20%20
            (Niagara|ResetSystem (Variables|Default|GetNG_Splash))
            (if (== _result (Variables|Default|GetmaxPos))
              (Variables|Default|SetcurrentPos 0))))))
    (else
      (CallFunction|Initialize) ; In case not init after first frame
      (goto _label))))

(fn ConstructionScript)

(fn Initialize
  (LocalVariables|SetPositions (Variables|/Game/Blueprints/MiniGames/DyeMaker/GM_Dyemaker_2D.GM_Dyemaker_2D_C|GetPositions (Variables|Default|GetGameMode)))
  (Variables|Default|SethasPositions (Utilities|Array|IsNotEmpty (LocalVariables|GetPositions)))
  (Variables|Default|SettimeTillBeat (/ 6e+01 72.0))
  (Variables|Default|SetmaxPos (Utilities|Array|Length (LocalVariables|GetPositions)))
  (Variables|Default|SetcurrentPos (Utilities|Array|LastIndex (LocalVariables|GetPositions))))