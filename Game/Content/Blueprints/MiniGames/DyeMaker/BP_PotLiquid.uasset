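; Pot liquid sprite actor for the DyeMaker minigame that shifts color while Zen is active.
; It listens to the Zen activation event on GM_Dyemaker_2D and targets the ColorList entry one above the current PurityLevel.
; Tick linearly blends the sprite color over the maximum Zen duration, restarting the blend if Zen outlasts it.
; Deactivation stops blending and makes the target the next start color.
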(event Custom|ZenActivated
  (params (IsActive :type Boolean))
  (CallFunction|SetNewColors IsActive))

(event EventBeginPlay
  (bind _asgm_dyemaker_2d (Utilities|Casting|CastToGM_Dyemaker_2D (Game|GetGameMode)))
  (Variables|Default|SetGMDyeMaker _asgm_dyemaker_2d)
  (EventDispatchers|BindEventtoOnZenActivated (Variables|Default|GetGMDyeMaker) (delegate Custom|ZenActivated))
  (Variables|Default|SettimeTillBeat (Default|GetZenDurationMax (Variables|Default|GetGMDyeMaker)))
  (bind _output_get (Variables|Default|SetSprite%20Color (Variables|/Script/Paper2D.PaperSpriteComponent|GetSpriteColor (Variables|Default|GetPaperSprite))))
  (Variables|Default|SetstartColor _output_get))

(event Collision|EventActorBeginOverlap
  (params (OtherActor :type Actor%20Object%20Reference)))

(event EventTick
  (params (DeltaSeconds :type Float%20%28single-precision%29))
  (bind _startcolor (Variables|Default|GetstartColor))
  (bind _endcolor (Variables|Default|GetendColor))
  (bind (_r _g _b) (Utilities|Struct|BreakLinearColor _endcolor))
  (bind (_r_2 _g_2 _b_2) (Utilities|Struct|BreakLinearColor _startcolor))
  (if (Variables|Default|GetchangeColor)
    (Variables|Default|SetcurrentTime (+ DeltaSeconds (Variables|Default|GetcurrentTime)))
    (if (<= (Variables|Default|GetcurrentTime) (Variables|Default|GettimeTillBeat))
      (Sprite|SetSpriteColor (Variables|Default|GetPaperSprite) (Utilities|Struct|MakeLinearColor (Math|Interpolation|Ease "Linear" (/ (Variables|Default|GetcurrentTime) (Variables|Default|GettimeTillBeat)) _r_2 _r) (Math|Interpolation|Ease "Linear" (/ (Variables|Default|GetcurrentTime) (Variables|Default|GettimeTillBeat)) _g_2 _g) (Math|Interpolation|Ease "Linear" (/ (Variables|Default|GetcurrentTime) (Variables|Default|GettimeTillBeat)) _b_2 _b) 255.0))
      (else
        (Variables|Default|SetcurrentTime 0.0)))))

(fn ConstructionScript)

(fn SetNewColors
  (params (zenActivated :type Boolean))
  (Utilities|String|LogString (Utilities|String|Append "ZEN FROM LIQUID. ACTIVE STATE: " (Utilities|String|ToString(Boolean) zenActivated)))
  (if zenActivated
    (Variables|Default|SetendColor (Utilities|Array|Get(acopy) (Variables|Default|GetcolorList) (+ (Variables|/Game/Blueprints/MiniGames/DyeMaker/GM_Dyemaker_2D.GM_Dyemaker_2D_C|GetPurityLevel (Variables|Default|GetGMDyeMaker)) 1)))
    (Variables|Default|SetchangeColor true)
    (else
      (Variables|Default|SetchangeColor false)
      (Variables|Default|SetstartColor (Variables|Default|GetendColor))))
  (Variables|Default|SetcurrentTime 0.0))