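; BP_Score is a short-lived text popup that rates a beat hit in the DyeMaker minigame.
; UpdateScore shows "perfect" or "nice" by absolute timing offset, with a larger size for perfect, or ".." on a miss; the "good" branch is unreachable.
; Tick steadily shrinks the TextRender's scale, and the actor destroys itself one second after BeginPlay.
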(event EventBeginPlay
  (Utilities|FlowControl|Delay 1.0)
  (Actor|DestroyActor))

(event Collision|EventActorBeginOverlap
  (params (OtherActor :type Actor%20Object%20Reference)))

(event EventTick
  (params (DeltaSeconds :type Float%20%28single-precision%29))
  (bind _output_get (Variables|Default|SetstartScale (- (Variables|Default|GetstartScale) (/ DeltaSeconds 1e+01))))
  (Transformation|SetRelativeScale3D (Variables|Default|GetTextRender) (Math|Vector|MakeVector _output_get _output_get _output_get)))

(fn ConstructionScript)

(fn UpdateScore
  (params (delayForScoring :type Float%20%28double-precision%29) (beatSuccess :type Boolean))
  (bind _textrender (Variables|Default|GetTextRender))
  (Utilities|FlowControl|Sequence
    (:then_0
      (if beatSuccess
        (bind _output_get (LocalVariables|SetabsDelay (Math|Float|Absolute(Float) delayForScoring)))
        (if (Math|Float|InRange(Float) _output_get 0.0 0.1)
          (LocalVariables|Setscoretext "perfect")
          (LocalVariables|SetfinalSize 15.0)
          (else
            (LocalVariables|Setscoretext "nice")
            (LocalVariables|SetfinalSize 1e+01)))
        (else
          (LocalVariables|Setscoretext ".."))))
    (:then_1
      (Rendering|Components|TextRender|SetText _textrender (Utilities|Text|ToText(String) (LocalVariables|Getscoretext)))
      (Rendering|Components|TextRender|SetWorldSize _textrender (LocalVariables|GetfinalSize)))))