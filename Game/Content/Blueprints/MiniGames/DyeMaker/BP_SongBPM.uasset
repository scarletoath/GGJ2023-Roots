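; Beat sequencer for the DyeMaker rhythm minigame, spawning timed BP_BeatIndicator targets from a BPM and song map DataTable.
; Each table row is a four-beat-long bar, evenly subdivided by its BeatList length, and Tick counts through beats until rows run out.
; Indicators appear at cycling or random positions, move Stick there, and enable scoring three beat intervals later.
; The oldest indicator explodes as a miss at MaxPositions, or as a hit through DestroySomething.
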(event Custom|SpawnNextBeat
  (params (spawnLoc :type Transform) (random :type Boolean))
  (bind _returnvalue (Math|Random|RandomUnitVector))
  (bind _returnvalue_2 (Math|Random|RandomFloatinRange 1e+02 4e+02))
  (bind _spawnedactors (Variables|Default|GetspawnedActors))
  (bind _returnvalue_3 (* _returnvalue _returnvalue_2))
  (bind (_x _y) (Math|Vector|BreakVector _returnvalue_3))
  (if random
    (Variables|Default|SetspawnLoc (Math|Transform|MakeTransform (Math|Vector|MakeVector _x _y 0.0)))
    (else
      (Variables|Default|SetspawnLoc spawnLoc)))
  (bind _returnvalue_4 (Game|SpawnActorfromClass "/Game/Blueprints/MiniGames/DyeMaker/BP_BeatIndicator.BP_BeatIndicator_C" (Variables|Default|GetspawnLoc) "Undefined" 0 0))
  (Default|EnableScoreonDelay _returnvalue_4 (* (Variables|Default|GetdelayPerBeat) 3.0))
  (bind _returnvalue_5 (Utilities|Array|Add (Variables|Default|GetspawnedActors) _returnvalue_4))
  (Transformation|SetActorLocation (Variables|Default|Getstick) (Transformation|GetWorldLocation (Variables|/Script/Engine.Actor|GetRootComponent _returnvalue_4)) false false)
  (if (== (Variables|Default|GetmaxPositions) _returnvalue_5)
    (bind _output_get (Variables|Default|SetactorToDestroy (Utilities|Array|Get(acopy) _spawnedactors)))
    (Utilities|Array|RemoveItem _spawnedactors _output_get)
    (bind _asbp_beat_indicator (Utilities|Casting|CastToBP_BeatIndicator _output_get))
    (Default|Kaboom _asbp_beat_indicator false))
  (Math|Integer|IncrementInt (Variables|Default|GetpositionCount)
    (:%20%20
      (if (> (Variables|Default|GetpositionCount) (- (Utilities|Array|Length (Variables|Default|Getpositions)) 1))
        (Variables|Default|SetpositionCount 0)))))

(event EventBeginPlay
  (bind _output_get (Variables|Default|SetdelayPerBeat (/ 6e+01 (Math|Conversions|ToFloat(Integer) (Variables|Default|GetBPM)))))
  (Variables|Default|SettimePerBar (* _output_get 4.0))
  (bind _outrownames (DataTable|GetDataTableRowNames (Variables|Default|GetsongMap)))
  (Utilities|String|LogString (Utilities|String|Append "TOTAL BARS_" (Utilities|String|ToString(Integer) (Utilities|Array|Length _outrownames))))
  (Variables|Default|SetbeatsInBar (CallFunction|UpdateBeatsinBar)))

(event EventTick
  (params (DeltaSeconds :type Float%20%28single-precision%29))
  (if (not (Variables|Default|GetsongEnd))
    (Variables|Default|SetcurrentTime (+ DeltaSeconds (Variables|Default|GetcurrentTime)))
    (if (>= (Variables|Default|GetcurrentTime) (Variables|Default|GetdelayPerBeat))
      (Variables|Default|SetcurrentTime 0.0)
      (Math|Integer|IncrementInt (Variables|Default|GetbeatNumber)
        (:%20%20
          (Utilities|FlowControl|Sequence
            (:then_0
              (if (> (Variables|Default|GetbeatNumber) (Variables|Default|GetbeatsInBar))
                (Variables|Default|SetbeatNumber 1)
                (Math|Integer|IncrementInt (Variables|Default|GetbarNumber)
                  (:%20%20
                    (Variables|Default|SetbeatsInBar (CallFunction|UpdateBeatsinBar))))))
            (:then_1
              (if (not (Variables|Default|GetsongEnd))
                (Utilities|String|LogString (Utilities|String|Append "BEAT! " "Beat No." (Utilities|String|ToString(Integer) (Variables|Default|GetbeatNumber)) "_Bar No." (Utilities|String|ToString(Integer) (Variables|Default|GetbarNumber))))
                (CallFunction|SpawnNextBeat (Transformation|GetActorTransform (Utilities|Array|Get(acopy) (Variables|Default|Getpositions) (Variables|Default|GetpositionCount))) (Variables|Default|GetRandom))))))))))

(fn UpdateBeatsinBar
  (bind _outrownames (DataTable|GetDataTableRowNames (Variables|Default|GetsongMap)))
  (bind _returnvalue (Utilities|GetDataTableRow (Variables|Default|GetsongMap) (Utilities|Array|Get(acopy) _outrownames (- (Variables|Default|GetbarNumber) 1)))
    (:then
      (bind _output_get (LocalVariables|SetnumBeats (Utilities|Array|Length (.BeatList (Utilities|Struct|BreakSTR_Bar _returnvalue)))))
      (bind _output_get_2 (Variables|Default|SetdelayPerBeat (/ (Variables|Default|GettimePerBar) _output_get)))
      (Utilities|String|LogString (Utilities|String|Append "DELAY PER BEAT: " (Utilities|String|ToString(Float) _output_get_2)))
      (return (LocalVariables|GetnumBeats)))
    (:RowNotFound
      (Utilities|String|LogString "Song end")
      (Variables|Default|SetsongEnd true))))

(fn DestroySomething
  (bind _spawnedactors (Variables|Default|GetspawnedActors))
  (Utilities|String|LogString "destroy something")
  (if (> (Utilities|Array|Length (Variables|Default|GetspawnedActors)) 0)
    (bind _output_get (LocalVariables|SetspacebarDestroy (Utilities|Array|Get(acopy) _spawnedactors)))
    (Utilities|Array|RemoveItem _spawnedactors _output_get)
    (bind _asbp_beat_indicator (Utilities|Casting|CastToBP_BeatIndicator _output_get))
    (Default|Kaboom _asbp_beat_indicator true)))