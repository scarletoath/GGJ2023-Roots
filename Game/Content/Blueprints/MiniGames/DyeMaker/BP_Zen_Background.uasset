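; Pulsing backdrop actor for the DyeMaker minigame's Zen mode, hidden until activated.
; It binds to the Dyemaker game mode's Zen activation event to toggle visibility.
; Tick restarts an expo-out ease on a 72 BPM beat, scaling the Paper sprite between Start and End while fading it from white to cyan.
; Disconnected nodes for cycling through a position list remain unused.
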(event Custom|OnZenActivated_Event
  (params (IsActive :type Boolean))
  (CallFunction|SetActive IsActive))

(event EventBeginPlay
  (Variables|Default|SettimeTillBeat (/ 6e+01 72.0))
  (Variables|Default|Setr (/ 2e+01 255.0))
  (Variables|Default|Setg (/ 2.2e+02 255.0))
  (Variables|Default|Setb (/ 254.0 255.0))
  (bind _asgm_dyemaker_2d (Utilities|Casting|CastToGM_Dyemaker_2D (Game|GetGameMode)))
  (EventDispatchers|BindEventtoOnZenActivated _asgm_dyemaker_2d (delegate Custom|OnZenActivated_Event))
  (CallFunction|SetActive false))

(event Collision|EventActorBeginOverlap
  (params (OtherActor :type Actor%20Object%20Reference)))

(event EventTick
  (params (DeltaSeconds :type Float%20%28single-precision%29))
  (bind _papersprite (Variables|Default|GetPaperSprite))
  (Variables|Default|SetcurrentTime (+ DeltaSeconds (Variables|Default|GetcurrentTime)))
  (if (<= (Variables|Default|GetcurrentTime) (Variables|Default|GettimeTillBeat))
    (Transformation|SetRelativeScale3D _papersprite (Math|Vector|MakeVector (Math|Interpolation|Ease "ExpoOut" (/ (Variables|Default|GetcurrentTime) (Variables|Default|GettimeTillBeat)) (Variables|Default|Getstart) (Variables|Default|Getend)) (Math|Interpolation|Ease "ExpoOut" (/ (Variables|Default|GetcurrentTime) (Variables|Default|GettimeTillBeat)) (Variables|Default|Getstart) (Variables|Default|Getend)) (Math|Interpolation|Ease "ExpoOut" (/ (Variables|Default|GetcurrentTime) (Variables|Default|GettimeTillBeat)) (Variables|Default|Getstart) (Variables|Default|Getend))))
    (Sprite|SetSpriteColor _papersprite (Math|Color|MakeColor (Math|Interpolation|Ease "ExpoOut" (/ (Variables|Default|GetcurrentTime) (Variables|Default|GettimeTillBeat)) 1.0 (Variables|Default|Getr)) (Math|Interpolation|Ease "ExpoOut" (/ (Variables|Default|GetcurrentTime) (Variables|Default|GettimeTillBeat)) 1.0 (Variables|Default|Getg)) (Math|Interpolation|Ease "ExpoOut" (/ (Variables|Default|GetcurrentTime) (Variables|Default|GettimeTillBeat)) 1.0 (Variables|Default|Getb))))
    (else
      (Variables|Default|SetcurrentTime 0.0))))

(fn ConstructionScript)

(fn SetActive
  (params (IsVisible :type Boolean))
  (Rendering|SetVisibility (Variables|Default|GetDefaultSceneRoot) IsVisible true))