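; Game mode for the 2D DyeMaker rhythm minigame, tracking Zen, timing accuracy and dye purity.
; BeginPlay caches name-sorted transforms of actors under "positionsRoot" and initializes the beat stick.
; A full Zen meter starts a timed Zen mode, during which accuracy derives from accumulated delay versus beat time.
; When Zen expires, purity level rises, with bonus points for meeting the data-table accuracy threshold.
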(event EventBeginPlay
  (Utilities|FlowControl|Sequence
    (:then_0
      (bind _positions (CallFunction|FindPositions))
      (Variables|Default|SetPositions _positions))
    (:then_1
      (bind _returnvalue (Actor|GetActorOfClass "/Game/Blueprints/MiniGames/DyeMaker/BP_BeatStick_2D.BP_BeatStick_2D_C"))
      (Default|Initialize _returnvalue))))

(event EventTick
  (params (DeltaSeconds :type Float%20%28single-precision%29))
  (if (CallFunction|IsZenActive)
    ;[1 1 1] Zen Active Duration Countdown
    (Variables|Default|SetZenDurationRemaining (Math|Float|Max(Float) (- (Variables|Default|GetZenDurationRemaining) DeltaSeconds) 0.0))
    ;[1 1 1] Deactivate on Time Up
    (if (not (CallFunction|IsZenActive))
      (CallFunction|ActivateZenMode false true))
    (else
      ;[1 1 1] Check Zen Progress and Activate
      (if (>= (Variables|Default|GetZenPercent) 1.0)
        (CallFunction|ActivateZenMode true false)))))

(fn ConstructionScript)

(fn FindPositions
  (bind _temppositions (LocalVariables|GettempPositions))
  (bind _actors (LocalVariables|Getactors))
  (Utilities|FlowControl|Sequence
    (:then_0
      (bind _outactors (Actor|GetAllActorswithTag "positionsRoot"))
      ;[1 1 1] Get actors with tag, and all their children. Insert at Sorted by name.
      (for _array_element _outactors
        (for _array_element_2 (Actor|GetAttachedActors _array_element true false)
          (bind (_array_element_3 _array_index) (Utilities|Array|ForEachLoopwithBreak (LocalVariables|Getactors) :!label _label)
            (:LoopBody
              (if (not (CallFunction|IsStringALessThanStringB (Utilities|GetDisplayName _array_element_3) (Utilities|GetDisplayName _array_element_2)))
                (LocalVariables|SetinsertIndex _array_index) ; Found insert index so stop finding
                (goto _label Break)))
            (:Completed
              (Utilities|Array|Insert _actors _array_element_2 (LocalVariables|GetinsertIndex))
              (LocalVariables|SetinsertIndex (Utilities|Array|Length _actors)) ; Default is add to end of array
            )))))
    (:then_1
      ;[1 1 1] Get Positions from Actors
      (for _array_element_4 (LocalVariables|Getactors)
        (Utilities|Array|Add _temppositions (Transformation|GetActorTransform _array_element_4)))
      (return _temppositions))))

(fn IsZenActive
  (return (> (Variables|Default|GetZenDurationRemaining) 0.0)))

(fn ActivateZenMode
  (params (IsActive :type Boolean) (UpdatePurity :type Boolean))
  (if IsActive
    (Variables|Default|SetZenDurationRemaining (Variables|Default|GetZenDurationMax))
    (CallFunction|ResetAccuracy)
    (Default|CallOnZenActivated IsActive :!label _label)
    (else
      (Variables|Default|SetZenPercent 0.0)
      ;[1 1 1] Increase Purity by 1 on Zen Completion. 1 or 2 points given into purity points based on acc
      (if UpdatePurity
        (bind _isaccurate (CallFunction|IsHighZenAccuracy))
        (Default|CallOnZenAccuracyCheck _isaccurate)
        (Variables|Default|SetPurityPoints (+ (select _isaccurate 2 1) (Variables|Default|GetPurityPoints)))
        (Math|Integer|IncrementInt (Variables|Default|GetPurityLevel)
          (:%20%20
            (goto _label)))))))

(fn IsHighZenAccuracy
  (bind _output (CallFunction|GetMinAccuracyforPurityLevel -1))
  (return (>= (Variables|Default|GetZenAccuracy) _output)))

(fn GetMinAccuracyforPurityLevel
  (params (PurityLevel :type Integer))
  (bind _datarow (CallFunction|GetPurityReqbyIndex "/Game/Blueprints/MiniGames/DyeMaker/Data/Data_PurityRequirements.Data_PurityRequirements" (Math|Integer|SelectInt (Variables|Default|GetPurityLevel) PurityLevel (< PurityLevel 0)) true))
  (return (Utilities|Struct|BreakSTR_PurityRequirement _datarow)))

(fn IncreaseZen
  (params (Percent :type Float%20%28double-precision%29))
  (Variables|Default|SetZenPercent (Math|Float|Clamp(Float) (+ (/ (Math|Float|Clamp(Float) Percent 0.0 1e+02) 1e+02) (Variables|Default|GetZenPercent))))
  (return (CallFunction|IsZenActive)))

(fn CalculateDyePurity
  (Utilities|String|LogString "CREATING DYE :D" false)
  (bind _returnvalue (UserInterface|CreateWidget "/Game/Blueprints/MiniGames/DyeMaker/UI_Dyemaker_Score.UI_Dyemaker_Score_C"))
  (UserInterface|Viewport|AddtoViewport _returnvalue 0))

(fn SetSongElapsed
  (params (percent :type Float%20%28double-precision%29))
  (Variables|Default|SetsongElapsed percent))

(fn UpdateAccuracy
  (params (delay :type Float%20%28double-precision%29) (beatTime :type Float%20%28double-precision%29))
  (bind _result (Math|Integer|IncrementInt (Variables|Default|GetZenBeatsPlayed))
    (:%20%20
      (Variables|Default|SetZenTotalBeatTime (* _result beatTime))
      (Variables|Default|SetZenTotalDelay (+ delay (Variables|Default|GetZenTotalDelay)))
      (Variables|Default|SetZenAccuracy (* (/ (- (Variables|Default|GetZenTotalBeatTime) (Variables|Default|GetZenTotalDelay)) (Variables|Default|GetZenTotalBeatTime)) 1e+02)))))

(fn ResetAccuracy
  (Variables|Default|SetZenAccuracy 0.0)
  (Variables|Default|SetZenTotalDelay 0.0)
  (Variables|Default|SetZenTotalBeatTime 0.0)
  (Variables|Default|SetZenBeatsPlayed 0))

(fn GetBarTime
  (return (* (Variables|Default|GettimePerBeat) 4.0)))

(fn GetZenTime
  (return (/ (Variables|Default|GetZenDurationRemaining) (Variables|Default|GetZenDurationMax))))