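; Utility function library for data table lookups, input key display info and string ordering.
; Purity requirement and key getters fetch rows by index, with optional clamping, or at random for keys.
; Key display info maps a key's long display name to a label and sprite row in Data_KeyDisplayInfos.
; The string comparison is a case-insensitive, character-code lexicographic less-than, with the shorter string first on a shared prefix.
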(fn GetPurityReqbyIndex
  (params (DataTable :type Data%20Table%20Object%20Reference) (Index :type Integer) (Clamp :type Boolean))
  (Utilities|FlowControl|Sequence
    (:then_0
      ;[1 1 1] Cache local vars
      (bind _output_get (LocalVariables|SetTable DataTable))
      (bind _outrownames (DataTable|GetDataTableRowNames _output_get))
      (LocalVariables|SetRowNames _outrownames))
    (:then_1
      ;[1 1 1] Clamp index if needed
      (if Clamp
        (LocalVariables|SetActualIndex (Math|Integer|Clamp(Integer) Index 0 (Utilities|Array|LastIndex (LocalVariables|GetRowNames))))
        (else
          (LocalVariables|SetActualIndex Index))))
    (:then_2
      (if (or Clamp (Utilities|Array|IsValidIndex (LocalVariables|GetRowNames) (LocalVariables|GetActualIndex)))
        ;[1 1 1] Actually Get Data
        (bind _returnvalue (Utilities|GetDataTableRow (LocalVariables|GetTable) (Utilities|Array|Get(acopy) (LocalVariables|GetRowNames) (LocalVariables|GetActualIndex)))
          (:then
            _)))
      (return _returnvalue))))

(fn GetKeysbyIndex
  (params (DataTable :type Data%20Table%20Object%20Reference) (Index :type Integer) (Clamp :type Boolean))
  (Utilities|FlowControl|Sequence
    (:then_0
      ;[1 1 1] Cache local vars
      (bind _output_get (LocalVariables|SetTable DataTable))
      (bind _outrownames (DataTable|GetDataTableRowNames _output_get))
      (LocalVariables|SetRowNames _outrownames))
    (:then_1
      ;[1 1 1] Clamp index if needed
      (if Clamp
        (LocalVariables|SetActualIndex (Math|Integer|Clamp(Integer) Index 0 (Utilities|Array|LastIndex (LocalVariables|GetRowNames))))
        (else
          (LocalVariables|SetActualIndex Index))))
    (:then_2
      (if (or Clamp (Utilities|Array|IsValidIndex (LocalVariables|GetRowNames) (LocalVariables|GetActualIndex)))
        ;[1 1 1] Actually Get Data
        (bind _returnvalue (Utilities|GetDataTableRow (LocalVariables|GetTable) (Utilities|Array|Get(acopy) (LocalVariables|GetRowNames) (LocalVariables|GetActualIndex)))
          (:then
            _)))
      (return _returnvalue))))

(fn GetRandomKeys
  (params (DataTable :type Data%20Table%20Object%20Reference))
  (bind _outrownames (DataTable|GetDataTableRowNames DataTable))
  ;[1 1 1] Actually Get Data
  (bind _returnvalue (Utilities|GetDataTableRow DataTable (.OutItem (Utilities|Array|Random _outrownames)))
    (:then
      (return _returnvalue))))

(fn GetKeyDisplayInfo
  (params (Key :type Key%20Structure :default "None"))
  (bind _returnvalue (Utilities|GetDataTableRow "/Game/Blueprints/MiniGames/DyeMaker/Data_KeyDisplayInfos.Data_KeyDisplayInfos" (Utilities|String|StringToName (Utilities|String|Replace (Utilities|String|ToString(Text) (Class|KismetInputLibrary|KeyGetDisplayName Key true)) " ")))
    (:then
      _)
    (:RowNotFound
      _))
  (return (.Label (Utilities|Struct|BreakSTR_KeyDisplayInfo _returnvalue)) (.Sprite (Utilities|Struct|BreakSTR_KeyDisplayInfo _returnvalue))))

(fn IsStringALessThanStringB
  (params (A :type String) (B :type String))
  (Utilities|FlowControl|Sequence
    (:then_0
      ;[0 0.05118 1] Convert each string to lower case and store as an array of characters
      (bind _output_get (LocalVariables|SetLocalA (Utilities|String|ToLower A)))
      (LocalVariables|SetLocalArrayA (Utilities|String|GetCharacterArrayfromString _output_get)))
    (:then_1
      (bind _output_get_2 (LocalVariables|SetLocalB (Utilities|String|ToLower B)))
      (LocalVariables|SetLocalArrayB (Utilities|String|GetCharacterArrayfromString _output_get_2)))
    (:then_2
      ;[0 1 0.004274] Get the length of each string
      (LocalVariables|SetLocalLengthA (Utilities|Array|Length (LocalVariables|GetLocalArrayA)))
      (LocalVariables|SetLocalLengthB (Utilities|Array|Length (LocalVariables|GetLocalArrayB))))
    (:then_3
      ;[0.9427 1 0] Determine the number of iterations of the next FOR LOOP (the length of whichever string is shorter)
      (if (<= (LocalVariables|GetLocalLengthA) (LocalVariables|GetLocalLengthB))
        (LocalVariables|SetCount (LocalVariables|GetLocalLengthA))
        (else
          (LocalVariables|SetCount (LocalVariables|GetLocalLengthB)))))
    (:then_4
      ;[1 0 0.0222] For each character convert it to its ascii number and compare the numbers
      (bind _result (Math|Integer|DecrementInt (LocalVariables|GetCount))
        (:%20%20
          (for _index (range 0 _result)
            (if (< (Utilities|String|GetCharacterasNumber (LocalVariables|GetLocalA) _index) (Utilities|String|GetCharacterasNumber (LocalVariables|GetLocalB) _index))
              (return true)
              (elif (not (== (Utilities|String|GetCharacterasNumber (LocalVariables|GetLocalA) _index) (Utilities|String|GetCharacterasNumber (LocalVariables|GetLocalB) _index)))
                (return false))))
          (if (== (LocalVariables|GetLocalLengthA) (LocalVariables|GetLocalLengthB))
            (return false) ; Strings are equal
            (elif (< (LocalVariables|GetLocalLengthA) (LocalVariables|GetLocalLengthB))
              (return true) ; StringA is less than StringB
              (else
                (return false) ; StringA is greater than StringB
              ))))))))