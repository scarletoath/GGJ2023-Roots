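; BP_BeatStick is an actor that moves between a list of marker positions in time with a fixed 72 BPM beat.
; Each Tick linearly interpolates its location from the current PosList entry to the next over one beat, wrapping back to the first.
; When a beat elapses, it resets the timer, advances the index and restarts the NGSplash effect.
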(event EventBeginPlay
  (Variables|Default|SethasPositions (> (Utilities|Array|Length (Variables|Default|GetposList)) 0))
  (Variables|Default|SettimeTillBeat (/ 6e+01 72.0))
  (Variables|Default|SetmaxPos (Utilities|Array|Length (Variables|Default|GetposList))))

(event Collision|EventActorBeginOverlap
  (params (OtherActor :type Actor%20Object%20Reference)))

(event EventTick
  (params (DeltaSeconds :type Float%20%28single-precision%29))
  (if (Variables|Default|GethasPositions)
    (Variables|Default|SetcurrentTime (+ DeltaSeconds (Variables|Default|GetcurrentTime)))
    (if (<= (Variables|Default|GetcurrentTime) (Variables|Default|GettimeTillBeat))
      (Transformation|SetActorLocation (.Location (Math|Transform|BreakTransform (Math|Interpolation|Ease "Linear" (/ (Variables|Default|GetcurrentTime) (Variables|Default|GettimeTillBeat)) (Transformation|GetActorTransform (Utilities|Array|Get(acopy) (Variables|Default|GetposList) (Variables|Default|GetcurrentPos))) (Transformation|GetActorTransform (Utilities|Array|Get(acopy) (Variables|Default|GetposList) (Math|Integer|SelectInt (+ (Variables|Default|GetcurrentPos) 1) 0 (< (+ (Variables|Default|GetcurrentPos) 1) (Variables|Default|GetmaxPos)))))))) false false)
      (else
        (Variables|Default|SetcurrentTime 0.0)
        (bind _result (Math|Integer|IncrementInt (Variables|Default|GetcurrentPos))
          (:%20%20
            (Niagara|ResetSystem (Variables|Default|GetNG_Splash))
            (if (== _result (Variables|Default|GetmaxPos))
              (Variables|Default|SetcurrentPos 0))))))))

(fn ConstructionScript)