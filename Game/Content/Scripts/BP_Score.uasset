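; BP_Score is a short-lived text popup actor that shows feedback on the result of a beat.
; UpdateScore picks a rating word from the beat success flag and whether the score is positive, then applies it to the TextRender with a color from an unassigned local variable.
; Tick steadily shrinks the text's uniform scale, and BeginPlay destroys the actor after a brief delay.
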(event EventBeginPlay
  (Utilities|FlowControl|Delay 1.0)
  (Actor|DestroyActor))

(event Collision|EventActorBeginOverlap
  (params (OtherActor :type Actor%20Object%20Reference)))

(event EventTick
  (params (DeltaSeconds :type Float%20%28single-precision%29))
  (bind _output_get (Variables|Default|SetstartScale (- (Variables|Default|GetstartScale) (/ DeltaSeconds 1e+01))))
  (Transformation|SetRelativeScale3D (Variables|Default|GetTextRender) (Math|Vector|MakeVector _output_get _output_get _output_get)))

(fn ConstructionScript)

(fn UpdateScore
  (params (score :type Float%20%28double-precision%29) (beatSuccess :type Boolean))
  (bind _textrender (Variables|Default|GetTextRender))
  (if beatSuccess
    (if (> score 0.0)
      (LocalVariables|Setscoretext "nice")
      (else
        (LocalVariables|Setscoretext "good")))
    (else
      (LocalVariables|Setscoretext "..")))
  (Rendering|Components|TextRender|SetText _textrender (Utilities|Text|ToText(String) (LocalVariables|Getscoretext)))
  (Rendering|Components|TextRender|SetTextRenderColor _textrender (LocalVariables|GetNewLocalVar)))