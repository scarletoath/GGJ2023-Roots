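; BP_Song is an actor that starts a song after a bar-based delay and shows a beat countdown.
; On BeginPlay it derives the delay from BPSongBPM's bar length, BarDelay and Offset, then plays the Cue as 2D sound.
; Tick shrinks the Countdown text, updating its number and setting full scale each beat, though StartScale itself never resets.
; Space Bar calls DestroySomething on BPSongBPM.
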(event EventBeginPlay
  (Variables|Default|SetstartDelay (+ (* (Variables|/Game/Scripts/BP_SongBPM.BP_SongBPM_C|GettimePerBar (Variables|Default|GetBP_SongBPM)) (Variables|Default|GetbarDelay)) (Variables|Default|Getoffset)))
  (Utilities|FlowControl|Delay (Variables|Default|GetstartDelay))
  (Audio|PlaySound2D (Variables|Default|Getcue) 1.0 1.0 0.0 0 0))

(event Collision|EventActorBeginOverlap
  (params (OtherActor :type Actor%20Object%20Reference)))

(event EventTick
  (params (DeltaSeconds :type Float%20%28single-precision%29))
  (if (> (Variables|Default|GetbeatCount) 0)
    (bind _output_get (Variables|Default|SetcountdownTime (+ DeltaSeconds (Variables|Default|GetcountdownTime))))
    (if (>= _output_get (Variables|/Game/Scripts/BP_SongBPM.BP_SongBPM_C|GetdelayPerBeat (Variables|Default|GetBP_SongBPM)))
      (Transformation|SetRelativeScale3D (Variables|Default|Getcountdown) "1.000000,1.000000,1.000000")
      (bind _result (Math|Integer|DecrementInt (Variables|Default|GetbeatCount))
        (:%20%20
          (Rendering|Components|TextRender|SetText (Variables|Default|Getcountdown) (Utilities|Text|ToText(Integer) _result))
          (Variables|Default|SetcountdownTime 0.0)))
      (else
        (bind _output_get_2 (Variables|Default|SetstartScale (- (Variables|Default|GetstartScale) (/ DeltaSeconds 1e+01))))
        (Transformation|SetRelativeScale3D (Variables|Default|Getcountdown) (Math|Vector|MakeVector _output_get_2 _output_get_2 _output_get_2))))))

(event Input|KeyboardEvents|SpaceBar
  (params (Key :type Key%20Structure :default "None"))
  (:Pressed
    (Default|DestroySomething (Variables|Default|GetBP_SongBPM))))

(fn ConstructionScript)