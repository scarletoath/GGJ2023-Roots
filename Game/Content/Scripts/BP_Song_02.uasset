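; Rhythm game song controller that spawns beat indicators in time with Canon in D and scores Space bar presses.
; Tick counts beats, spacing each bar from BPM and its SongMap row's beat count, while music starts after a bar delay plus offset.
; Indicators cycle through Positions and enable scoring three beats later.
; Presses score the oldest indicator, scaling ScoreCube; exceeding the threshold resets score and plays the Zen track.
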(event EventBeginPlay
  (bind _output_get (Variables|Default|SetdelayPerBeat (/ 6e+01 (Math|Conversions|ToFloat(Integer) (Variables|Default|GetBPM)))))
  (Variables|Default|SettimePerBar (* _output_get 4.0))
  (DataTable|GetDataTableRowNames (Variables|Default|GetsongMap))
  (Variables|Default|SetbeatsInBar (CallFunction|UpdateBeatsinBar))
  (Variables|Default|SetstartDelay (+ (* (Variables|Default|GettimePerBar) (Variables|Default|GetbarDelay)) (Variables|Default|Getoffset)))
  (Utilities|FlowControl|Delay (Variables|Default|GetstartDelay))
  (bind _returnvalue (Audio|CreateSound2D "/Game/Assets/bgm_Canon_in_D_Cue_BASE.bgm_Canon_in_D_Cue_BASE" 1.0 1.0 0.0 0))
  (bind _output_get_2 (Variables|Default|SetAudioSource _returnvalue))
  (Audio|Components|Audio|Play _output_get_2 0.0)
  (bind _returnvalue_2 (Audio|CreateSound2D "/Game/Assets/bgm_Canon_in_D_1_Cue_ZEN.bgm_Canon_in_D_1_Cue_ZEN" 1.0 1.0 0.0 0))
  (Variables|Default|SetAudioSource2 _returnvalue_2))

(event Collision|EventActorBeginOverlap
  (params (OtherActor :type Actor%20Object%20Reference)))

(event EventTick
  (params (DeltaSeconds :type Float%20%28single-precision%29))
  (if (not (Variables|Default|GetsongEnd))
    (Variables|Default|SetcurrentTime (+ DeltaSeconds (Variables|Default|GetcurrentTime)))
    (if (>= (Variables|Default|GetcurrentTime) (Variables|Default|GetdelayPerBeat))
      (Variables|Default|SetcurrentTime 0.0)
      (Math|Integer|IncrementInt (Variables|Default|GetbeatNumber)
        (:%20%20
          (Utilities|FlowControl|Sequence
            (:then_0
              (if (> (Variables|Default|GetbeatNumber) (Variables|Default|GetbeatsInBar))
                (Variables|Default|SetbeatNumber 1)
                (Math|Integer|IncrementInt (Variables|Default|GetbarNumber)
                  (:%20%20
                    (Variables|Default|SetbeatsInBar (CallFunction|UpdateBeatsinBar))))))
            (:then_1
              (if (not (Variables|Default|GetsongEnd))
                (Utilities|String|LogString (Utilities|String|Append "BEAT! " "Beat No." (Utilities|String|ToString(Integer) (Variables|Default|GetbeatNumber)) "_Bar No." (Utilities|String|ToString(Integer) (Variables|Default|GetbarNumber))))
                (CallFunction|CreateBeat (Transformation|GetActorTransform (Utilities|Array|Get(acopy) (Variables|Default|Getpositions) (Variables|Default|GetpositionCount))))))))))))

(event Input|KeyboardEvents|SpaceBar
  (params (Key :type Key%20Structure :default "None"))
  (:Pressed
    (CallFunction|ScoreLatestBeat)))

(fn ConstructionScript)

(fn UpdateBeatsinBar
  (bind _outrownames (DataTable|GetDataTableRowNames (Variables|Default|GetsongMap)))
  (bind _returnvalue (Utilities|GetDataTableRow (Variables|Default|GetsongMap) (Utilities|Array|Get(acopy) _outrownames (- (Variables|Default|GetbarNumber) 1)))
    (:then
      (bind _output_get (Variables|Default|SetnumBeats (Utilities|Array|Length (.BeatList (Utilities|Struct|BreakSTR_Bar _returnvalue)))))
      (bind _output_get_2 (Variables|Default|SetdelayPerBeat (/ (Variables|Default|GettimePerBar) _output_get)))
      (Utilities|String|LogString (Utilities|String|Append "DELAY PER BEAT: " (Utilities|String|ToString(Float) _output_get_2)))
      (return (Variables|Default|GetnumBeats)))
    (:RowNotFound
      (Utilities|String|LogString "Song end")
      (Variables|Default|SetsongEnd true))))

(fn CreateBeat
  (params (transform :type Transform))
  (bind _returnvalue (Math|Random|RandomUnitVector))
  (bind _returnvalue_2 (Math|Random|RandomFloatinRange 1e+02 4e+02))
  (bind _returnvalue_3 (* _returnvalue _returnvalue_2))
  (bind (_x _y) (Math|Vector|BreakVector _returnvalue_3))
  (if false
    (LocalVariables|SetspawnLoc (Math|Transform|MakeTransform (Math|Vector|MakeVector _x _y 0.0)))
    (else
      (LocalVariables|SetspawnLoc transform)))
  (bind _returnvalue_4 (Game|SpawnActorfromClass "/Game/Scripts/BP_BeatIndicator.BP_BeatIndicator_C" (LocalVariables|GetspawnLoc) "Undefined" 0 0))
  (Default|EnableScoreonDelay _returnvalue_4 (* (Variables|Default|GetdelayPerBeat) 3.0))
  (Utilities|Array|Add (Variables|Default|GetspawnedActors) _returnvalue_4)
  (Math|Integer|IncrementInt (Variables|Default|GetpositionCount)
    (:%20%20
      (if (> (Variables|Default|GetpositionCount) (- (Utilities|Array|Length (Variables|Default|Getpositions)) 1))
        (Variables|Default|SetpositionCount 0)))))

(fn ScoreLatestBeat
  (bind _spawnedactors (Variables|Default|GetspawnedActors))
  (bind _output (Utilities|Array|Get(acopy) _spawnedactors))
  (LocalVariables|SetobjectToScore _output)
  (bind _asbp_beat_indicator (Utilities|Casting|CastToBP_BeatIndicator _output))
  (bind _finalscoredelay (Default|Kaboom _asbp_beat_indicator true))
  (Variables|Default|SetcurrentScore (+ (CallFunction|CalculateScore _finalscoredelay) (Variables|Default|GetcurrentScore)))
  (Transformation|SetActorScale3D (Variables|Default|GetscoreCube) (Math|Vector|MakeVector (Variables|Default|GetcurrentScore) 1.0 1.0))
  (Utilities|Array|RemoveItem (Variables|Default|GetspawnedActors) (LocalVariables|GetobjectToScore))
  (if (> (Variables|Default|GetcurrentScore) 5.0)
    (Variables|Default|SetcurrentScore 0.0)
    (Variables|Default|SetzenMode true)
    (Audio|Components|Audio|Play (Variables|Default|GetAudioSource2) 4e+01)))

(fn CalculateScore
  (params (scoreDelay :type Float%20%28double-precision%29))
  (bind _output_get (LocalVariables|SetscoreToCalculate scoreDelay))
  (if (< _output_get 0.0)
    (LocalVariables|SetscoreToReward 0.2)
    (elif (> (LocalVariables|GetscoreToCalculate) 0.2)
      (LocalVariables|SetscoreToReward 0.3)
      (else
        (LocalVariables|SetscoreToReward 1.0))))
  (return (LocalVariables|GetscoreToReward)))